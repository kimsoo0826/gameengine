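; Enemy actor for a shooter game that takes damage and hurts the hero while overlapping it.
; DecreaseHP lowers its health and, at zero or below, tells the cached shooter game mode to increase score and decrease the enemy count, then destroys the actor.
; Overlap with heroBp deals damage immediately and starts a looping timer that repeats the hit through a DecreaseHP message until the overlap ends.
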(event Custom|decreaseheroBP
  (Class|Damage|DecreaseHP(Message) (stale Collision|EventActorBeginOverlap _ashero_bp) 3e+01))

(event EventBeginPlay
  (Variables|Default|SetHP 1e+02)
  (bind _asshooter (Utilities|Casting|CastToshooter (Game|GetGameMode)))
  (Variables|Default|Setgamemode _asshooter))

(event Collision|EventActorBeginOverlap
  (params (OtherActor :type Actor%20Object%20Reference))
  (bind _ashero_bp (Utilities|Casting|CastToheroBp OtherActor))
  (CallFunction|DecreaseheroBP)
  (Utilities|Time|SetTimerbyFunctionName 0 "decreaseheroBP" 0.33 true))

(event EventTick
  (params (DeltaSeconds :type Float%20%28single-precision%29)))

(event Collision|EventActorEndOverlap
  (params (OtherActor :type Actor%20Object%20Reference))
  (Utilities|Casting|CastToheroBp OtherActor)
  (Utilities|Time|ClearTimerbyFunctionName 0 "decreaseheroBP"))

(event EventDecreaseHP
  (params (amount :type Float%20%28single-precision%29))
  (bind _gamemode (Variables|Default|Getgamemode))
  (bind _output_get (Variables|Default|SetHP (- (Variables|Default|GetHP) amount)))
  (if (<= _output_get 0.0)
    (Default|IncreaseScore _gamemode)
    (Default|DecreaseEnemy _gamemode)
    (Actor|DestroyActor)))

(fn ConstructionScript)