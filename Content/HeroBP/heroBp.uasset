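; Player hero character for a shooter, with world-axis movement, yaw turning and a health pool.
; On BeginPlay it caches the shooter GameMode, sets full HP, then spawns a GunBP and snaps its mesh to the character's Mesh.
; The trigger input starts and stops the gun firing.
; DecreaseHP updates the GameMode's UI and, at zero HP, hides the capsule and its children, then restarts the level by console command after a short delay.
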(event EventBeginPlay
  (bind _asshooter (Utilities|Casting|CastToshooter (Game|GetGameMode)))
  (Variables|Default|Setgame%20mode _asshooter)
  (Variables|Default|SetheroHP 1e+02)
  (bind _returnvalue (Game|SpawnActorfromClass "/Game/gunBP/gunBP.gunBP_C" (Transformation|GetWorldTransform (Variables|Character|GetMesh)) "Undefined" 0 0))
  (bind _output_get (Variables|Default|Setgun _returnvalue))
  (Transformation|AttachComponentToComponent (Variables|/Game/gunBP/gunBP.gunBP_C|GetSK_FPGun _output_get) (Variables|Character|GetMesh) "None" "SnapToTarget" "SnapToTarget" "KeepWorld" true))

(event Collision|EventActorBeginOverlap
  (params (OtherActor :type Actor%20Object%20Reference)))

(event EventTick
  (params (DeltaSeconds :type Float%20%28single-precision%29)))

(event EventDecreaseHP
  (params (amount :type Float%20%28single-precision%29))
  (bind _output_get (Variables|Default|SetheroHP (- (Variables|Default|GetheroHP) amount)))
  (Default|Updataherohp (Variables|/Game/shooter.shooter_C|GetgameUI (Variables|Default|Getgame%20mode)) _output_get)
  (Development|PrintString (Utilities|String|ToString(Float) _output_get))
  (if (<= _output_get 0.0)
    (Rendering|SetVisibility (Variables|Collision|GetCapsuleComponent) false true)
    (Utilities|FlowControl|Delay 0.2)
    (Development|ExecuteConsoleCommand "restartlevel")))

(event Input|ActionEvents|InputActiontriggerbullet
  (params (Key :type Key%20Structure :default "AnyKey"))
  (bind _gun (Variables|Default|Getgun))
  (:Pressed
    (Default|StartFiring _gun))
  (:Released
    (Default|Stopfiring _gun)))

(event Input|AxisEvents|InputAxismoveforward
  (params (AxisValue :type Float%20%28single-precision%29))
  (Pawn|Input|AddMovementInput "1.000000, 0, 0" AxisValue false))

(event Input|AxisEvents|InputAxismoveright
  (params (AxisValue :type Float%20%28single-precision%29))
  (Pawn|Input|AddMovementInput "0,1.000000, 0" AxisValue false))

(event Input|AxisEvents|InputAxisturnright
  (params (AxisValue :type Float%20%28single-precision%29))
  (Transformation|AddActorLocalRotation (Math|Rotator|MakeRotator 0.0 0.0 (* AxisValue 3.0)) false false))

(fn ConstructionScript)