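; HeroBP is the player hero, which moves along world axes, turns by yaw input and shoots with a gun.
; On BeginPlay it shows the cursor, initializes HP, and spawns a MousePointBP marker and a Gun attached to the mesh's GunSocket.
; Left click moves the marker to the cursor trace hit, sets Ispunching and starts firing until release.
; DecreaseHP subtracts damage and restarts the level after a short delay when HP runs out.
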(event EventBeginPlay
  (bind _returnvalue (Game|SpawnActorfromClass "/Game/UI/MousePointBP.MousePointBP_C" (Math|Conversions|ToTransform(Vector) (Transformation|GetActorLocation)) "Undefined" 0 0))
  (Variables|Default|SetMouseClickPoint _returnvalue)
  (Variables|/Script/Engine.PlayerController|SetbShowMouseCursor (Game|GetPlayerController 0) true)
  (Variables|Default|SetheroHP 1e+01)
  (bind _returnvalue_2 (Game|SpawnActorfromClass "/Game/gun/gun.gun_C" (Transformation|GetWorldTransform (Variables|Character|GetMesh)) "Undefined" 0 0))
  (bind _output_get (Variables|Default|Setgun _returnvalue_2))
  (Transformation|AttachComponentToComponent (Variables|/Game/gun/gun.gun_C|GetSK_FPGun _output_get) (Variables|Character|GetMesh) "GunSocket" "SnapToTarget" "SnapToTarget" "KeepWorld" true))

(event Collision|EventActorBeginOverlap
  (params (OtherActor :type Actor%20Object%20Reference)))

(event EventDecreaseHP
  (params (amount :type Float%20%28single-precision%29))
  (bind _output_get (Variables|Default|SetheroHP (- (Variables|Default|GetheroHP) amount)))
  (if (<= _output_get 0.0)
    (Utilities|FlowControl|Delay 1.0)
    (Development|ExecuteConsoleCommand "RestartLevel")))

(event EventTick
  (params (DeltaSeconds :type Float%20%28single-precision%29)))

(event Input|ActionEvents|InputActionLeftMouseClicked
  (params (Key :type Key%20Structure :default "AnyKey"))
  (bind _returnvalue (Game|GetPlayerController 0))
  (bind _gun (Variables|Default|Getgun))
  (bind _hitresult (Game|Player|GetHitResultUnderCursorbyChannel _returnvalue "TraceTypeQuery1" true))
  (bind _location (Collision|BreakHitResult _hitresult))
  (:Pressed
    (Variables|Default|Setispunching true)
    (Transformation|SetActorLocation (Variables|Default|GetMouseClickPoint) (Math|Vector|MakeVector (.x _location) (.y _location) (.z _location)) false false)
    (Default|StartFire _gun))
  (:Released
    (Variables|Default|Setispunching false)
    (Default|StopFire _gun)))

(event Input|AxisEvents|InputAxisforward
  (params (AxisValue :type Float%20%28single-precision%29))
  (Pawn|Input|AddMovementInput "1.000000, 0, 0" AxisValue false))

(event Input|AxisEvents|InputAxisturn
  (params (AxisValue :type Float%20%28single-precision%29))
  (Transformation|AddActorLocalRotation (Math|Rotator|MakeRotator 0.0 0.0 (* AxisValue 3.0)) false false))

(event Input|AxisEvents|InputAxisbackward
  (params (AxisValue :type Float%20%28single-precision%29))
  (Pawn|Input|AddMovementInput "1.000000, 0, 0" AxisValue false))

(event Input|AxisEvents|InputAxisright
  (params (AxisValue :type Float%20%28single-precision%29))
  (Pawn|Input|AddMovementInput "0,1.000000, 0" AxisValue false))

(event Input|AxisEvents|InputAxisleft
  (params (AxisValue :type Float%20%28single-precision%29))
  (Pawn|Input|AddMovementInput "0,1.000000, 0" AxisValue false))

(fn ConstructionScript)