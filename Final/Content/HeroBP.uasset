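; HeroBP is a player-controlled hero with axis-driven movement and a mouse-click point marker.
; On BeginPlay it spawns a MousePointBP at its own location and shows the mouse cursor.
; A left click moves that marker to the Visibility trace hit under the cursor; the hero itself does not move toward it.
; Movement inputs follow fixed world X/Y axes, independent of the yaw applied by the turn axis.
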(event EventBeginPlay
  (bind _returnvalue (Game|SpawnActorfromClass "/Game/UI/MousePointBP.MousePointBP_C" (Math|Conversions|ToTransform(Vector) (Transformation|GetActorLocation)) "Undefined" 0 0))
  (Variables|Default|SetMouseClickPoint _returnvalue)
  (Variables|/Script/Engine.PlayerController|SetbShowMouseCursor (Game|GetPlayerController 0) true))

(event Collision|EventActorBeginOverlap
  (params (OtherActor :type Actor%20Object%20Reference)))

(event EventTick
  (params (DeltaSeconds :type Float%20%28single-precision%29)))

(event Input|ActionEvents|InputActionLeftMouseClicked
  (params (Key :type Key%20Structure :default "AnyKey"))
  (:Pressed
    (Transformation|SetActorLocation (Variables|Default|GetMouseClickPoint) (.Location (Collision|BreakHitResult (.HitResult (Game|Player|GetHitResultUnderCursorbyChannel (Game|GetPlayerController 0) "TraceTypeQuery1" true)))) false false)))

(event Input|AxisEvents|InputAxisforward
  (params (AxisValue :type Float%20%28single-precision%29))
  (Pawn|Input|AddMovementInput "1.000000, 0, 0" AxisValue false))

(event Input|AxisEvents|InputAxisturn
  (params (AxisValue :type Float%20%28single-precision%29))
  (Transformation|AddActorLocalRotation (Math|Rotator|MakeRotator 0.0 0.0 (* AxisValue 3.0)) false false))

(event Input|AxisEvents|InputAxisbackward
  (params (AxisValue :type Float%20%28single-precision%29))
  (Pawn|Input|AddMovementInput "1.000000, 0, 0" AxisValue false))

(event Input|AxisEvents|InputAxisright
  (params (AxisValue :type Float%20%28single-precision%29))
  (Pawn|Input|AddMovementInput "0,1.000000, 0" AxisValue false))

(event Input|AxisEvents|InputAxisleft
  (params (AxisValue :type Float%20%28single-precision%29))
  (Pawn|Input|AddMovementInput "0,1.000000, 0" AxisValue false))

(fn ConstructionScript)