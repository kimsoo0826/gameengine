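; Enemy actor Blueprint that damages the hero on contact and destroys itself when its own health runs out.
; HP is set at BeginPlay and reduced by a DecreaseHP event.
; Overlapping a HeroBP applies damage immediately and starts a looping timer that repeats it through DecreaseHPMessage.
; Ending the overlap clears that timer by function name.
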(event Custom|decreaseHeroHP
  (Class|Damageinterface|DecreaseHP(Message) (stale Collision|EventActorBeginOverlap _ashero_bp) 3e+01))

(event EventBeginPlay
  (Variables|Default|SetHP 1e+02))

(event Collision|EventActorBeginOverlap
  (params (OtherActor :type Actor%20Object%20Reference))
  (bind _ashero_bp (Utilities|Casting|CastToHeroBP OtherActor))
  (CallFunction|DecreaseHeroHP)
  (Utilities|Time|SetTimerbyFunctionName 0 "decreaseHeroHP" 0.33 true))

(event EventDecreaseHP
  (params (amount :type Float%20%28single-precision%29))
  (bind _output_get (Variables|Default|SetHP (- (Variables|Default|GetHP) amount)))
  (if (<= _output_get 0.0)
    (Actor|DestroyActor)))

(event Collision|EventActorEndOverlap
  (params (OtherActor :type Actor%20Object%20Reference))
  (Utilities|Casting|CastToHeroBP OtherActor)
  (Utilities|Time|ClearTimerbyFunctionName 0 "decreaseHeroHP"))

(event EventTick
  (params (DeltaSeconds :type Float%20%28single-precision%29)))

(fn ConstructionScript)